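; Spawner actor that fills the level with Asteroid1 actors, each launched in a random direction in the XZ plane.
; While the stored count is below 20, Tick drives a two-second Delay that spawns one at a fixed location with random pitch and a strong impulse.
; The count is refreshed from GetAllActorsOfClass and printed only after each spawn, so spawning stops for good once it reaches the cap.
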(event `self.ReceiveBeginPlay`)

(event `self.ReceiveActorBeginOverlap`
  (params (OtherActor :type "Actor Object Reference")))

(event `self.ReceiveTick`
  (params (DeltaSeconds :type "Float (single-precision)"))
  (bind _returnvalue (`KismetMathLibrary.MakeRot` (.pitch (`KismetMathLibrary.RandomRotator` false))))
  (if (< (`self.AsteroidCount`) 20)
    (`KismetSystemLibrary.Delay` 2.0)
    (bind _returnvalue_2 (`|SpawnActorFromClass` "/Game/Blueprints/Asteroid1.Asteroid1_C" (`KismetMathLibrary.MakeTransform` (100.0 0.0 100.0) _returnvalue (1.0 1.0 1.0))))
    (`PrimitiveComponent.AddImpulse` _returnvalue_2 (`KismetMathLibrary.GreaterGreater_VectorRotator` (80000.0 0.0 0.0) _returnvalue) "None" false)
    (bind _outactors (`GameplayStatics.GetAllActorsOfClass` "/Game/Blueprints/Asteroid1.Asteroid1_C"))
    (bind _output_get (set `self.AsteroidCount` (`KismetArrayLibrary.Array_Length` _outactors)))
    (`KismetSystemLibrary.PrintString` (`KismetStringLibrary.Concat_StrStr` "Number of Asteriods: " (`KismetStringLibrary.Conv_IntToString` _output_get)))))

(fn `UserConstructionScript`)