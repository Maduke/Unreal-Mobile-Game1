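; MyHUD is a HUD Blueprint that displays the player's score at the top center of the screen.
; Its DrawHUD event casts the player pawn to PlayerObj, reads Score and draws it as green labeled text in the Comic_Andy font.
; GetTextSize measures the string so it stays horizontally centered as the value changes.
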(event `self.ReceiveBeginPlay`)

(event `self.ReceiveActorBeginOverlap`
  (params (OtherActor :type "Actor Object Reference")))

(event `self.ReceiveTick`
  (params (DeltaSeconds :type "Float (single-precision)")))

(event `self.ReceiveDrawHUD`
  (params (SizeX :type Integer) (SizeY :type Integer))
  ;[1 1 1] Draw the player's Score to the HUD
  (bind _asplayer_obj (cast `/Game/Blueprints/PlayerObj` (`GameplayStatics.GetPlayerPawn` 0)))
  (bind _returnvalue (`KismetStringLibrary.Concat_StrStr` "Score: " (`KismetStringLibrary.Conv_IntToString` (`/Game/Blueprints/PlayerObj.Score` _asplayer_obj))))
  (`self.DrawText` _returnvalue (struct :`G` 1.5 :`B` 0.279649 :`A` 1.0) (- (`KismetMathLibrary.Conv_IntToDouble` (/ SizeX 2)) (/ (`self.GetTextSize` _returnvalue "/Game/Fonts/Comic_Andy.Comic_Andy") 2.0)) (`KismetMathLibrary.Conv_IntToDouble` 20) "/Game/Fonts/Comic_Andy.Comic_Andy" 1.0))

(fn `UserConstructionScript`)