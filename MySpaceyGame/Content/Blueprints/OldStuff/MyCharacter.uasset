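; A 2D flipbook character Blueprint with side-scrolling movement along X and hold-to-fire ball shooting.
; While left mouse is held, Tick passes through a short delay to spawn MyBall ahead, spending Ammo1.
; Space only adds diagonal movement input, and the facing check compares two constants, so never turns.
; An Idle/Running/Jumping flipbook selector exists, but its update, Jump and replication setup are disconnected.
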(event Custom|UpdateAnimation
  ;[1 1 1] Animate
)

(event EventBeginPlay
  ;[1 1 1] Replication
)

(event EventActorBeginOverlap
  (params (OtherActor :type Actor%20Object%20Reference)))

(event EventTick
  (params (DeltaSeconds :type Float%20%28single-precision%29))
  (bind _returnvalue (Transformation|GetActorRotation))
  ;[1 1 1] Shoot balls
  (if (Variables|Default|GetCanShoot)
    (Utilities|FlowControl|Delay 0.2)
    (if (> (Variables|Default|GetAmmo1) 0)
      (Game|SpawnActorfromClass "/Game/Blueprints/MyBall.MyBall_C" (Math|Transform|MakeTransform (+ (Transformation|GetActorLocation) (* (Math|Vector|GetForwardVector _returnvalue) 1e+02) (* (Math|Vector|GetUpVector _returnvalue) 5e+01)) _returnvalue "0.200000,0.200000,0.200000") false 0)
      (Variables|Default|SetAmmo1 (- (Variables|Default|GetAmmo1) 1)))))

(event Input|ActionEvents|InputActionJump
  ;[1 1 1] Jumping
)

(event Input|AxisEvents|InputAxisMoveRight
  (params (AxisValue :type Float%20%28single-precision%29))
  ;[1 1 1] Movement
  (Pawn|Input|AddMovementInput "1.000000, 0,0.000000" AxisValue false)
  (CallFunction|UpdateAnimation)
  (Math|Float|CompareFloat 0.0 0.0
    (:>
      (Pawn|SetControlRotation (Pawn|GetController) (Class|KismetMathLibrary|MakeRot 0.0 0.0 0.0)))
    (:<
      (Pawn|SetControlRotation (Pawn|GetController) (Class|KismetMathLibrary|MakeRot 0.0 1.8e+02 0.0)))))

(event Input|MouseEvents|LeftMouseButton
  ;[1 1 1] Shoot balls
  (:Pressed
    (Variables|Default|SetCanShoot true))
  (:Released
    (Variables|Default|SetCanShoot false)))

(event Input|KeyboardEvents|SpaceBar
  (:Pressed
    (Pawn|Input|AddMovementInput "1.000000,0.000000,1.000000" 1.0 false)))

(fn ConstructionScript)

(fn AnimationStateMachine
  (params (IsFalling :type Boolean :default false) (IsMoving :type Boolean :default false))
  ;[1 1 1] collect data
  (LocalVariables|SetIsFallingLocal IsFalling)
  (LocalVariables|SetIsMovingLocal IsMoving)
  ;[1 1 1] Test Data
  (|TestForJumping
    (:then
      ;[1 1 1] Set Animation State
      (LocalVariables|SetAnimationState "NewEnumerator2"))
    (:else
      (|TestForRunningorIdle
        (:then
          (LocalVariables|SetAnimationState "NewEnumerator1"))
        (:else
          (LocalVariables|SetAnimationState "NewEnumerator0")))))
  (return (Utilities|Select :Index (LocalVariables|GetAnimationState) :NewEnumerator0 (Variables|Animation|GetIdleFlipbook) :NewEnumerator1 (Variables|Animation|GetRunFlipbook) :NewEnumerator2 (Variables|Animation|GetFallingFlipbook))))