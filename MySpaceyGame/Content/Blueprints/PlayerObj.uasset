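; Physics-driven sprite player object that turns with impulses and fires MyBall projectiles, tinting itself and showing the mouse cursor on begin play.
; While TestShoot is held, Tick spawns balls ahead of it, rate-limited by a CanShoot flag and ShootSpeed delay.
; Each shot pushes the player backward as recoil and launches the ball forward with a stronger impulse.
; TurnLeft and TurnRight axes apply opposite angular impulses around Y.
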(event `self.ReceiveBeginPlay`
  ;[1 1 1] Event Begin Play
  (`PaperFlipbookComponent.SetSpriteColor` (struct :`R` 100.0 :`G` 0.554772 :`B` 0.58 :`A` 1.0))
  (set `PlayerController.bShowMouseCursor` true (`GameplayStatics.GetPlayerController` 0)))

(event `self.ReceiveTick`
  (params (DeltaSeconds :type "Float (single-precision)"))
  (bind _returnvalue (`self.K2_GetActorRotation`))
  (bind _returnvalue_2 (`KismetMathLibrary.GreaterGreater_VectorRotator` (-15000.0 0.0 0.0) _returnvalue))
  ;[1 1 1] Control movement
  (if (`self.IsShooting`)
    (if (`self.CanShoot`)
      (set `self.CanShoot` false)
      (bind _returnvalue_3 (`|SpawnActorFromClass` "/Game/Blueprints/MyBall.MyBall_C" (`KismetMathLibrary.MakeTransform` (+ (`self.K2_GetActorLocation`) (* (`KismetMathLibrary.GetForwardVector` _returnvalue) 75.0)) (struct) (0.15 0.15 0.15)) true))
      (`PrimitiveComponent.AddImpulse` _returnvalue_2)
      (`PrimitiveComponent.AddImpulse` _returnvalue_3 (* _returnvalue_2 -6.0) "None" false)
      (`KismetSystemLibrary.Delay` (`self.ShootSpeed`))
      (set `self.CanShoot` true))))

(event `InputAction|TestShoot` :overrideparent false
  ;[1 1 1] Control movement
  (:`Pressed`
    (set `self.IsShooting` true))
  (:`Released`
    (set `self.IsShooting` false)))

(event `InputAxis|TurnLeft`
  (params (AxisValue :type "Float (single-precision)"))
  ;[1 1 1] Rotation Handling
  (if (> AxisValue 0.0)
    (bind _output_get (set `self.Steer` (* AxisValue -0.5)))
    (`PrimitiveComponent.AddAngularImpulse` (`KismetMathLibrary.MakeVector` 0.0 _output_get) "None" true)
    (else
      (set `self.Steer` 0.0))))

(event `InputAxis|TurnRight`
  (params (AxisValue :type "Float (single-precision)"))
  ;[1 1 1] Rotation Handling
  (if (> AxisValue 0.0)
    (bind _output_get (set `self.Steer` (* AxisValue 0.5)))
    (`PrimitiveComponent.AddAngularImpulse` (`KismetMathLibrary.MakeVector` 0.0 _output_get) "None" true)
    (else
      (set `self.Steer` 0.0))))

(fn `UserConstructionScript`)